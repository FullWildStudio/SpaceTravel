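; Player-controlled spaceship Blueprint that flies through physics forces driven by input axes.
; Roll, Pitch and Yaw each drive a pair of thruster components on the wings or nose and tail, setting strength from axis value and deactivating at zero.
; EngineThruster applies an impulse to the SpaceShip component along the ArrowPitch arrow's forward vector on each axis update, without delta-time scaling.
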(event EventBeginPlay)

(event Collision|EventActorBeginOverlap
  (params (OtherActor :type Actor%20Object%20Reference)))

(event EventTick
  (params (DeltaSeconds :type Float%20%28single-precision%29)))

(event Input|AxisEvents|InputAxisEngineThruster
  (params (AxisValue :type Float%20%28single-precision%29))
  (Physics|AddImpulse (Variables|Default|GetSpaceShip) (* (Math|Vector|GetForwardVector (Transformation|GetWorldRotation (Variables|Default|GetArrowPitch))) (* AxisValue (Variables|Default|GetEnginePower))) "None" false))

(event Input|AxisEvents|InputAxisRoll
  (params (AxisValue :type Float%20%28single-precision%29))
  (bind _rollstrength (Variables|Default|GetRollStrength))
  (bind _leftwingrollthrust (Variables|Default|GetLeftWingRollThrust))
  (bind _rightwingrollthrust (Variables|Default|GetRightWingRollThrust))
  (bind _returnvalue (* AxisValue _rollstrength))
  ;[1 1 1] Handling Roll
  (if (!= AxisValue 0.0)
    (Components|Activation|Activate _leftwingrollthrust false)
    (Components|Activation|Activate _rightwingrollthrust false)
    (Variables|/Script/Engine.PhysicsThrusterComponent|SetThrustStrength _leftwingrollthrust _returnvalue)
    (Variables|/Script/Engine.PhysicsThrusterComponent|SetThrustStrength _rightwingrollthrust _returnvalue)
    (else
      (Components|Activation|Deactivate (Variables|Default|GetLeftWingRollThrust))
      (Components|Activation|Deactivate (Variables|Default|GetRightWingRollThrust)))))

(event Input|AxisEvents|InputAxisPitch
  (params (AxisValue :type Float%20%28single-precision%29))
  (bind _pitchstrenght (Variables|Default|GetPitchStrenght))
  (bind _nosepitchthrust (Variables|Default|GetNosePitchThrust))
  (bind _tailpitchthrust (Variables|Default|GetTailPitchThrust))
  (bind _returnvalue (* AxisValue _pitchstrenght))
  ;[1 1 1] Handling Pitch
  (if (!= AxisValue 0.0)
    (Components|Activation|Activate _nosepitchthrust false)
    (Components|Activation|Activate _tailpitchthrust false)
    (Variables|/Script/Engine.PhysicsThrusterComponent|SetThrustStrength _nosepitchthrust _returnvalue)
    (Variables|/Script/Engine.PhysicsThrusterComponent|SetThrustStrength _tailpitchthrust _returnvalue)
    (else
      (Components|Activation|Deactivate (Variables|Default|GetNosePitchThrust))
      (Components|Activation|Deactivate (Variables|Default|GetTailPitchThrust)))))

(event Input|AxisEvents|InputAxisYaw
  (params (AxisValue :type Float%20%28single-precision%29))
  (bind _yawstrength (Variables|Default|GetYawStrength))
  (bind _noseyawthrust (Variables|Default|GetNoseYawThrust))
  (bind _tailyawthrust (Variables|Default|GetTailYawThrust))
  (bind _returnvalue (* AxisValue _yawstrength))
  ;[1 1 1] Handling Yaw
  (if (!= AxisValue 0.0)
    (Components|Activation|Activate _noseyawthrust false)
    (Components|Activation|Activate _tailyawthrust false)
    (Variables|/Script/Engine.PhysicsThrusterComponent|SetThrustStrength _noseyawthrust _returnvalue)
    (Variables|/Script/Engine.PhysicsThrusterComponent|SetThrustStrength _tailyawthrust _returnvalue)
    (else
      (Components|Activation|Deactivate (Variables|Default|GetNoseYawThrust))
      (Components|Activation|Deactivate (Variables|Default|GetTailYawThrust)))))

(fn ConstructionScript)