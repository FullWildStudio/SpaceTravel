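; BasicResource is an actor with a text render component, likely a base resource object, that spins continuously in the world.
; Each Tick rebuilds the actor transform, advancing yaw at a constant DeltaSeconds-scaled rate while zeroing pitch and roll and forcing unit scale.
; The construction script sets the text render color, and no overlap or pickup logic is implemented.
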(event EventBeginPlay)

(event Collision|EventActorBeginOverlap
  (params (OtherActor :type Actor%20Object%20Reference)))

(event EventTick
  (params (DeltaSeconds :type Float%20%28single-precision%29))
  (Transformation|SetActorTransform (Math|Transform|MakeTransform (Transformation|GetActorLocation) (Math|Rotator|MakeRotator 0.0 0.0 (+ (* DeltaSeconds 1e+02) (.Yaw (Math|Rotator|BreakRotator (Transformation|GetActorRotation))))))))

(fn ConstructionScript
  (Rendering|Components|TextRender|SetTextRenderColor (Variables|Default|GetTextRender) (Math|Color|MakeColor 0 0 0 1)))